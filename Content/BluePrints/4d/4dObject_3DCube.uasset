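; 3D cube variant of a 4D object, built as points at W = 0 joined by lines.
; The construction script generates corner coordinates, twice per corner due to an unused fourth loop, and assigns cube edge indices before running parent construction.
; Rotate turns every 4D point component, remapping XY, YZ and ZX planes to XW, YW and ZW, then updates the spline meshes.
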(event EventBeginPlay)

(event Collision|EventActorBeginOverlap
  (params (OtherActor :type Actor%20Object%20Reference)))

(event EventTick
  (params (DeltaSeconds :type Float%20%28single-precision%29))
  (|CallParentFunction 0.0))

(event EventRotate
  (params (RotationPlane :type 4dPlane%20Enum :default "NewEnumerator0") (Angle :type Float%20%28single-precision%29))
  (for _array_element (Variables|Default|Get4dPointCompReferences)
    (Default|Rotate _array_element (Utilities|Select :Index RotationPlane :NewEnumerator0 "NewEnumerator3" :NewEnumerator1 "NewEnumerator4" :NewEnumerator2 "NewEnumerator5" :NewEnumerator3 "NewEnumerator3" :NewEnumerator4 "NewEnumerator4" :NewEnumerator5 "NewEnumerator5") Angle))
  (CallFunction|UpdateSplineMesh))

(fn ConstructionScript
  (bind _vertices (Variables|Default|GetVertices))
  (bind _cubesize (Variables|Default|GetCubeSize))
  (for _index (range 0 1)
    (for _index_2 (range 0 1)
      (for _index_3 (range 0 1)
        (for _index_4 (range 0 1)
          (Utilities|Array|Add _vertices (- (* _index _cubesize) 5e+01))
          (Utilities|Array|Add _vertices (- (* _index_2 _cubesize) 5e+01))
          (Utilities|Array|Add _vertices (- (* _index_3 _cubesize) 5e+01))
          (Utilities|Array|Add _vertices 0.0)))))
  (Variables|Default|SetLineStartIndex (LocalVariables|GetCubeLineStart))
  (Variables|Default|SetLineEndIndex (LocalVariables|GetCubeLineEnd))
  (|CallParentFunction))