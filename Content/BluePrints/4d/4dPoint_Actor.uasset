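; 4dPoint_Actor is an actor that stores a point in four-dimensional space as X, Y, Z, W and provides functions to transform it.
; Translate offsets the coordinates by given deltas or by another point's components read through Break.
; Rotate writes sine and cosine into plane-specific slots of a flattened 4x4 matrix for one of six planes, then multiplies the coordinates by it.
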(event EventBeginPlay)

(event Collision|EventActorBeginOverlap
  (params (OtherActor :type Actor%20Object%20Reference)))

(event EventTick
  (params (DeltaSeconds :type Float%20%28single-precision%29)))

(fn ConstructionScript)

(fn Translate
  (params (dx :type Float%20%28single-precision%29) (dy :type Float%20%28single-precision%29) (dz :type Float%20%28single-precision%29) (dw :type Float%20%28single-precision%29))
  (Variables|Default|Setx (+ dx (Variables|Default|Getx)))
  (Variables|Default|Sety (+ dy (Variables|Default|Gety)))
  (Variables|Default|Setz (+ dz (Variables|Default|Getz)))
  (Variables|Default|Setw (+ dw (Variables|Default|Getw))))

(fn Break
  (return (Variables|Default|Getx) (Variables|Default|Gety) (Variables|Default|Getz) (Variables|Default|Getw)))

(fn Rotate
  (params (RotationPlane :type 4dPlane%20Enum) (Angle :type Float%20%28single-precision%29))
  (bind _returnvalue (Math|Trig|Sin(Degrees) Angle))
  (bind _returnvalue_2 (Math|Trig|Cos(Degrees) Angle))
  (bind _xyzwnew (LocalVariables|GetxyzwNew))
  (for (_array_element _array_index) (Utilities|Array|MakeArray _returnvalue_2 _returnvalue (* _returnvalue -1.0) _returnvalue_2)
    (Utilities|Array|SetArrayElem (LocalVariables|GetRotationMatrix) (Utilities|Array|Get(acopy) (Utilities|Select :Index RotationPlane :NewEnumerator0 (LocalVariables|GetXY) :NewEnumerator1 (LocalVariables|GetYZ) :NewEnumerator2 (LocalVariables|GetXZ) :NewEnumerator3 (LocalVariables|GetXW) :NewEnumerator4 (LocalVariables|GetYW) :NewEnumerator5 (LocalVariables|GetZW)) _array_index) _array_element))
  (LocalVariables|SetxyzwOriginal (Utilities|Array|MakeArray (Variables|Default|Getx) (Variables|Default|Gety) (Variables|Default|Getz) (Variables|Default|Getw)))
  (for _index (range 0 3)
    (LocalVariables|SettempValue 0.0)
    (for _index_2 (range 0 3)
      (LocalVariables|SettempValue (+ (LocalVariables|GettempValue) (* (Utilities|Array|Get(acopy) (LocalVariables|GetRotationMatrix) (+ (* _index 4) _index_2)) (Utilities|Array|Get(acopy) (LocalVariables|GetxyzwOriginal) _index_2)))))
    (Utilities|Array|Add (LocalVariables|GetxyzwNew) (LocalVariables|GettempValue)))
  (Variables|Default|Setx (Utilities|Array|Get(acopy) _xyzwnew))
  (Variables|Default|Sety (Utilities|Array|Get(acopy) _xyzwnew 1))
  (Variables|Default|Setz (Utilities|Array|Get(acopy) _xyzwnew 2))
  (Variables|Default|Setw (Utilities|Array|Get(acopy) _xyzwnew 3)))

(fn Translatewith4dPoint
  (params (T :type 4d%20Point%20Actor%20Object%20Reference))
  (bind (_x _y _z _w) (CallFunction|Break T))
  (CallFunction|Translate _x _y _z _w))