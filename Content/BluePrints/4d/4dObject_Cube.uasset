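; Construction-script Blueprint that defines a 4D hypercube (tesseract) as vertex and line data for a 4D object.
; Four nested binary loops generate the 16 corners, appending each as four consecutive floats in Vertices, scaled by CubeSize with a fixed offset.
; It copies CubeLineStart and CubeLineEnd into the line index variables, then calls the parent construction script.
; Its event graph holds only disabled placeholder events.
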(event EventBeginPlay)

(event Collision|EventActorBeginOverlap
  (params (OtherActor :type Actor%20Object%20Reference)))

(event EventTick
  (params (DeltaSeconds :type Float%20%28single-precision%29))
  (|CallParentFunction 0.0))

(fn ConstructionScript
  (bind _vertices (Variables|Default|GetVertices))
  (bind _cubesize (Variables|Default|GetCubeSize))
  (for _index (range 0 1)
    (for _index_2 (range 0 1)
      (for _index_3 (range 0 1)
        (for _index_4 (range 0 1)
          (Utilities|Array|Add _vertices (- (* _index _cubesize) 5e+01))
          (Utilities|Array|Add _vertices (- (* _index_2 _cubesize) 5e+01))
          (Utilities|Array|Add _vertices (- (* _index_3 _cubesize) 5e+01))
          (Utilities|Array|Add _vertices (- (* _index_4 _cubesize) 5e+01))))))
  (Variables|Default|SetLineStartIndex (LocalVariables|GetCubeLineStart))
  (Variables|Default|SetLineEndIndex (LocalVariables|GetCubeLineEnd))
  (|CallParentFunction))