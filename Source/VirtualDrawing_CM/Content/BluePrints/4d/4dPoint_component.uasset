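; Component that stores a point in 4D space as an XYZW array and provides functions to read, translate and rotate it.
; Translation accepts an array, four separate coordinates or another 4D point component, with the latter two feeding the array version.
; Rotation writes sine and cosine terms into a flattened 4x4 matrix at indices chosen by one of six rotation planes, then multiplies the point by it.
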(event EventBeginPlay)

(event EventTick
  (params (DeltaSeconds :type Float%20%28single-precision%29)))

(fn Break
  (bind _xyzw (Variables|Default|Getxyzw))
  (return (Utilities|Array|Get(acopy) _xyzw) (Utilities|Array|Get(acopy) _xyzw 1) (Utilities|Array|Get(acopy) _xyzw 2) (Utilities|Array|Get(acopy) _xyzw 3)))

(fn Translatewith4dPoint
  (params (4dPointComponent :type 4d%20Point%20Component%20Object%20Reference))
  (bind (_x _y _z _w) (CallFunction|Break 4dPointComponent))
  (CallFunction|Translate (Utilities|Array|MakeArray _x _y _z _w)))

(fn Translate
  (params (xyzw :type Array%20of%20Floats%20%28single-precision%29))
  (for (_array_element _array_index) (Variables|Default|Getxyzw)
    (Utilities|Array|SetArrayElem (Variables|Default|Getxyzw) _array_index (+ _array_element (Utilities|Array|Get(acopy) xyzw _array_index)))))

(fn TranslatewithXYZW
  (params (x :type Float%20%28single-precision%29) (y :type Float%20%28single-precision%29) (z :type Float%20%28single-precision%29) (w :type Float%20%28single-precision%29))
  (CallFunction|Translate (Utilities|Array|MakeArray x y z w)))

(fn Rotate
  (params (RotationPlane :type 4dPlane%20Enum) (Angle :type Float%20%28single-precision%29))
  (bind _returnvalue (Math|Trig|Sin(Degrees) Angle))
  (bind _returnvalue_2 (Math|Trig|Cos(Degrees) Angle))
  (for (_array_element _array_index) (Utilities|Array|MakeArray _returnvalue_2 _returnvalue (* _returnvalue -1.0) _returnvalue_2)
    (Utilities|Array|SetArrayElem (LocalVariables|GetRotationMatrix) (Utilities|Array|Get(acopy) (Utilities|Select :Index RotationPlane :NewEnumerator0 (LocalVariables|GetXY) :NewEnumerator1 (LocalVariables|GetYZ) :NewEnumerator2 (LocalVariables|GetXZ) :NewEnumerator3 (LocalVariables|GetXW) :NewEnumerator4 (LocalVariables|GetYW) :NewEnumerator5 (LocalVariables|GetZW)) _array_index) _array_element))
  (LocalVariables|SetxyzwOriginal (Variables|Default|Getxyzw))
  (for _index (range 0 3)
    (LocalVariables|SettempValue 0.0)
    (for _index_2 (range 0 3)
      (LocalVariables|SettempValue (+ (LocalVariables|GettempValue) (* (Utilities|Array|Get(acopy) (LocalVariables|GetRotationMatrix) (+ (* _index 4) _index_2)) (Utilities|Array|Get(acopy) (LocalVariables|GetxyzwOriginal) _index_2)))))
    (Utilities|Array|Add (LocalVariables|GetxyzwNew) (LocalVariables|GettempValue)))
  (Variables|Default|Setxyzw (LocalVariables|GetxyzwNew)))