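; Actor that displays a four-dimensional object as a 3D wireframe with an optional solid mesh.
; Construction builds 4D point components, spline-mesh edges and, if enabled, a procedural mesh using triangle indices from a topology text file.
; Translate and Rotate move the points, then reproject them via axonometric, oblique or perspective projection to update edges and mesh.
; SectionAtW computes constant-W slice points from triangle edges; its debug drawing is unconnected.
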(event EventBeginPlay)

(event Collision|EventActorBeginOverlap
  (params (OtherActor :type Actor%20Object%20Reference)))

(event EventTick
  (params (DeltaSeconds :type Float%20%28single-precision%29)))

(fn ConstructionScript
  (bind _meshmaterialinstance (Variables|Default|GetMeshMaterialInstance))
  (bind _linematerialinstance (Variables|Default|GetLineMaterialInstance))
  (bind _vertices (Variables|Default|GetVertices))
  (for _index (range 0 (/ (Utilities|Array|Length (Variables|Default|GetVertices)) 4))
    (bind _returnvalue (AddComponent|Add4dPointComponent (Utilities|Array|MakeArray (Utilities|Array|Get(acopy) _vertices (* _index 4)) (Utilities|Array|Get(acopy) _vertices (+ (* _index 4) 1)) (Utilities|Array|Get(acopy) _vertices (+ (* _index 4) 2)) (Utilities|Array|Get(acopy) _vertices (+ (* _index 4) 3)))))
    (Utilities|Array|Add (Variables|Default|Get4dPointCompReferences) _returnvalue))
  (for _array_element (Variables|Default|GetLineStartIndex)
    (bind _returnvalue_2 (AddComponent|AddSplineMeshComponent true))
    (Transformation|AttachComponentToComponent _returnvalue_2 (Variables|Default|GetDefaultSceneRoot) "None" "KeepRelative" "KeepRelative" "KeepRelative" true)
    (if (Utilities|IsValid _linematerialinstance)
      (Rendering|Material|SetMaterial _returnvalue_2 0 _linematerialinstance)))
  (if (Variables|Default|GetbHasMesh)
    (for _array_element_2 (Variables|Default|Get4dPointCompReferences)
      (bind _projectedlocation (CallFunction|Project4DPoint _array_element_2))
      (Utilities|Array|Add (LocalVariables|GetVectorWS) _projectedlocation))
    (for _array_element_3 (Utilities|String|ParseIntoArray (.SaveTextA (Class|ReadWriteLibrary|FileLoadString "Content\\4d\\4dcubetopology.txt")) " 
")
      (Utilities|Array|Add (Variables|Default|GetTrianglesIndex) (Math|Conversions|ToInteger(Byte) _array_element_3)))
    (bind _returnvalue_3 (AddComponent|AddProceduralMeshComponent false))
    (Class|ProceduralMeshComponent|CreateMeshSectionLinearColor _returnvalue_3 0 (LocalVariables|GetVectorWS) (Variables|Default|GetTrianglesIndex) 0 0 0 0 false)
    (Rendering|Material|SetMaterial _returnvalue_3 0 (select (Utilities|IsValid _meshmaterialinstance) _meshmaterialinstance (Variables|Default|GetDefaultMeshMaterial))))
  (CallFunction|UpdateSplineMesh))

(fn Project4DPoint
  (params (4dPoint :type 4d%20Point%20Component%20Object%20Reference))
  (bind (_x _y _z _w) (Default|Break 4dPoint))
  (bind _projectedlocation (CallFunction|ProjectVectorandW _w (Math|Vector|MakeVector _x _y _z)))
  (return _projectedlocation))

(fn Translate
  (params (InVector4 :type Array%20of%20Floats%20%28single-precision%29))
  (for _array_element (Variables|Default|Get4dPointCompReferences)
    (Default|Translate _array_element InVector4))
  (CallFunction|UpdateSplineMesh))

(fn UpdateSplineMesh
  (bind _vertexworldspace (LocalVariables|GetVertexWorldSpace))
  (for _array_element (Variables|Default|Get4dPointCompReferences)
    (bind _projectedlocation (CallFunction|Project4DPoint _array_element))
    (Utilities|Array|Add (LocalVariables|GetVertexWorldSpace) _projectedlocation))
  (if (Variables|Default|GetbHasMesh)
    (Class|ProceduralMeshComponent|UpdateMeshSectionLinearColor (Actor|GetComponentbyClass "/Script/ProceduralMeshComponent.ProceduralMeshComponent") 0 (LocalVariables|GetVertexWorldSpace)))
  (for (_array_element_2 _array_index) (Actor|GetComponentsByClass "/Script/Engine.SplineMeshComponent")
    (SplineMesh|SetStartandEnd _array_element_2 (Utilities|Array|Get(acopy) _vertexworldspace (Utilities|Array|Get(acopy) (Variables|Default|GetLineStartIndex) _array_index)) (- (Utilities|Array|Get(acopy) _vertexworldspace (Utilities|Array|Get(acopy) (Variables|Default|GetLineEndIndex) _array_index)) (Utilities|Array|Get(acopy) _vertexworldspace (Utilities|Array|Get(acopy) (Variables|Default|GetLineStartIndex) _array_index))) (Utilities|Array|Get(acopy) _vertexworldspace (Utilities|Array|Get(acopy) (Variables|Default|GetLineEndIndex) _array_index)) (- (Utilities|Array|Get(acopy) _vertexworldspace (Utilities|Array|Get(acopy) (Variables|Default|GetLineEndIndex) _array_index)) (Utilities|Array|Get(acopy) _vertexworldspace (Utilities|Array|Get(acopy) (Variables|Default|GetLineStartIndex) _array_index))) true :!class /Script/Engine.SplineMeshComponent)))

(fn Rotate
  (params (RotationPlane :type 4dPlane%20Enum) (Angle :type Float%20%28single-precision%29))
  (for _array_element (Variables|Default|Get4dPointCompReferences)
    (Default|Rotate _array_element (select (Variables|Default|GetbRotate4D) RotationPlane (Utilities|Select :Index RotationPlane :NewEnumerator0 "NewEnumerator3" :NewEnumerator1 "NewEnumerator4" :NewEnumerator2 "NewEnumerator5" :NewEnumerator3 "NewEnumerator3" :NewEnumerator4 "NewEnumerator4" :NewEnumerator5 "NewEnumerator5")) Angle))
  (CallFunction|UpdateSplineMesh))

(fn SectionatW
  (params (w :type Float%20%28single-precision%29))
  (bind _4dpointcompreferences (Variables|Default|Get4dPointCompReferences))
  (bind _trianglesindex (Variables|Default|GetTrianglesIndex))
  (LocalVariables|SetLocalW w)
  (for _index (range 0 (/ (Utilities|Array|Length (Variables|Default|GetTrianglesIndex)) 3))
    (bind (_worldlocation _isvalid) (CallFunction|SectionLine (LocalVariables|GetLocalW) (Utilities|Array|Get(acopy) _4dpointcompreferences (Utilities|Array|Get(acopy) _trianglesindex (* _index 3))) (Utilities|Array|Get(acopy) _4dpointcompreferences (Utilities|Array|Get(acopy) _trianglesindex (+ (* _index 3) 1)))))
    (if _isvalid
      (Utilities|Array|Add (LocalVariables|GetSectionLinePoints) _worldlocation))
    (bind (_worldlocation_2 _isvalid_2) (CallFunction|SectionLine (LocalVariables|GetLocalW) (Utilities|Array|Get(acopy) _4dpointcompreferences (Utilities|Array|Get(acopy) _trianglesindex (+ (* _index 3) 1))) (Utilities|Array|Get(acopy) _4dpointcompreferences (Utilities|Array|Get(acopy) _trianglesindex (+ (* _index 3) 2)))))
    (if _isvalid_2
      (Utilities|Array|Add (LocalVariables|GetSectionLinePoints) _worldlocation_2))
    (bind (_worldlocation_3 _isvalid_3) (CallFunction|SectionLine (LocalVariables|GetLocalW) (Utilities|Array|Get(acopy) _4dpointcompreferences (Utilities|Array|Get(acopy) _trianglesindex (+ (* _index 3) 2))) (Utilities|Array|Get(acopy) _4dpointcompreferences (Utilities|Array|Get(acopy) _trianglesindex (* _index 3)))))
    (if _isvalid_3
      (Utilities|Array|Add (LocalVariables|GetSectionLinePoints) _worldlocation_3)))
  (for (_array_element _array_index) (LocalVariables|GetSectionLinePoints)
    (bind _projectedlocation (CallFunction|ProjectVectorandW (LocalVariables|GetLocalW) _array_element))
    (Utilities|Array|SetArrayElem (LocalVariables|GetSectionLinePoints) _array_index _projectedlocation))
  (return (LocalVariables|GetSectionLinePoints)))

(fn SectionLine
  (params (W :type Float%20%28single-precision%29) (Start :type 4d%20Point%20Component%20Object%20Reference) (End :type 4d%20Point%20Component%20Object%20Reference))
  (bind (_x _y _z _w) (Default|Break Start))
  (bind (_x_2 _y_2 _z_2 _w_2) (Default|Break End))
  (if (and (> W (Math|Float|Min(Float) _w_2 _w)) (< W (Math|Float|Max(Float) _w _w_2)))
    (bind _output_get (LocalVariables|Sett (/ (- W _w_2) (- _w_2 _w))))
    (return (Math|Vector|MakeVector (+ (* (- _x_2 _x) _output_get) _x_2) (+ (* (- _y_2 _y) _output_get) _y_2) (+ (* (- _z_2 _z) _output_get) _z_2)) true)
    (else
      (return "0, 0, 0" false))))

(fn ProjectVectorandW
  (params (W :type Float%20%28single-precision%29) (xyz :type Vector))
  (bind _l1 (LocalVariables|GetL1))
  (switch Utilities|FlowControl|Switch|Switchon4DProjectionMode (Variables|Default|GetProjectionMode)
    (:NewEnumerator0
      (LocalVariables|SetReturnVector xyz))
    (:NewEnumerator1
      (LocalVariables|SetReturnVector (+ xyz (* "0.577350,0.577350,0.577350" W))))
    (:NewEnumerator2
      (LocalVariables|SetReturnVector (* xyz (/ (- _l1 5e+01) (- _l1 W))))))
  (return (LocalVariables|GetReturnVector)))

(fn SetLineMaterial
  (params (Material :type Material%20Object%20Reference))
  (Rendering|Material|SetMaterial (Actor|GetComponentsByClass self "/Script/Engine.SplineMeshComponent") 0 Material))

(fn SetMeshMaterial
  (params (Material :type Material%20Object%20Reference))
  (Rendering|Material|SetMaterial (Actor|GetComponentsByClass self "/Script/ProceduralMeshComponent.ProceduralMeshComponent") 0 Material))