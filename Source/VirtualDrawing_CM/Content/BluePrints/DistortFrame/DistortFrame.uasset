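; DistortFrame is a four-sided frame actor whose edges can be bent toward a point.
; The construction script builds straight spline mesh edges between consecutive Vertices, plus a procedural quad with collision and a black vertical-clipped material, re-created on every loop pass.
; SetTangentsToPoint converts a world target to local space and re-aims each edge's tangents through it, curving the splines while leaving corners and quad fixed.
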(event EventBeginPlay)

(event Collision|EventActorBeginOverlap
  (params (OtherActor :type Actor%20Object%20Reference)))

(event EventTick
  (params (DeltaSeconds :type Float%20%28single-precision%29)))

(fn ConstructionScript
  (for (_array_element _array_index) (Variables|Default|GetVertices)
    (bind _returnvalue (AddComponent|AddSplineMeshComponent false))
    (SplineMesh|SetStartandEnd _returnvalue _array_element (- (Utilities|Array|Get(acopy) (Variables|Default|GetVertices) (Math|Integer|%(Integer) (+ _array_index 1) 4)) _array_element) (Utilities|Array|Get(acopy) (Variables|Default|GetVertices) (Math|Integer|%(Integer) (+ _array_index 1) 4)) (- (Utilities|Array|Get(acopy) (Variables|Default|GetVertices) (Math|Integer|%(Integer) (+ _array_index 1) 4)) _array_element) true :!class /Script/Engine.SplineMeshComponent)
    (Utilities|Array|Add (Variables|Default|GetSplineMeshArray) _returnvalue)
    (bind _returnvalue_2 (AddComponent|AddProceduralMeshComponent false))
    (Class|ProceduralMeshComponent|CreateMeshSectionLinearColor _returnvalue_2 0 (Variables|Default|GetVertices) (Utilities|Array|MakeArray 0 1 2 2 3 0) 0 0 0 0 true)
    (Rendering|Material|SetMaterial _returnvalue_2 0 "/Game/BluePrints/DistortFrame/M_Black_VerticalClipped2.M_Black_VerticalClipped2")))

(fn SetTangentstoPoint
  (params (Target :type Vector))
  (bind _returnvalue (Transformation|GetActorTransform))
  (bind _returnvalue_2 (Math|Transform|InvertTransform _returnvalue))
  (bind _returnvalue_3 (Math|Transform|TransformLocation _returnvalue_2 Target))
  (for _array_element (Variables|Default|GetSplineMeshArray)
    (SplineMesh|SetStartandEnd _array_element (SplineMesh|GetStartPosition _array_element) (- _returnvalue_3 (SplineMesh|GetStartPosition _array_element)) (SplineMesh|GetEndPosition _array_element) (- (SplineMesh|GetEndPosition _array_element) _returnvalue_3) true :!class /Script/Engine.SplineMeshComponent)))