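; VR settings panel with 3D buttons and text labels for the Teleport, Scale and Drag move modes and the Server Control toggle.
; Trace start and leave events find a button's box by tag and swap its child mesh between blue and red materials.
; Clicks cycle the enum or flip the boolean in GameState, update the label and copy the value to GameInstance.
; Labels initialize from GameState one second after BeginPlay.
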(event Custom|TraceStart
  (params (Tag :type Name))
  (bind _asstatic_mesh_component (Utilities|Casting|CastToStaticMeshComponent (Components|GetChildComponent (Utilities|Array|Get(acopy) (Actor|GetComponentsbyTag "/Script/Engine.BoxComponent" Tag)) 0)))
  (Rendering|Material|SetMaterial _asstatic_mesh_component 0 "/Game/VR_Player/Blueprints/VR_Character/UI_Assets/M_Blue.M_Blue"))

(event Custom|TraceLeave
  (params (Tag :type Name))
  (bind _asstatic_mesh_component (Utilities|Casting|CastToStaticMeshComponent (Components|GetChildComponent (Utilities|Array|Get(acopy) (Actor|GetComponentsbyTag "/Script/Engine.BoxComponent" Tag)) 0)))
  (Rendering|Material|SetMaterial _asstatic_mesh_component 0 "/Game/VR_Player/Blueprints/VR_Character/UI_Assets/M_Red.M_Red"))

(event Custom|ClickButton
  (params (Tag :type Name))
  (switch name Tag
    (:TeleportMode
      (bind _asgame_state (Utilities|Casting|CastToGameState (Game|GetGameState)))
      (bind _output_get (Variables|/Game/VR_Player/Blueprints/VR_Character/GameState.GameState_C|SetTeleportMode _asgame_state (Utilities|Enum|ByteToEnumE_MoveMode (Math|Conversions|ToByte(Integer) (Math|Integer|%(Integer) (+ (Math|Conversions|ToInteger(Byte) (Variables|/Game/VR_Player/Blueprints/VR_Character/GameState.GameState_C|GetTeleportMode _asgame_state)) 1) (|GetNumEnumEntries))))))
      (Rendering|Components|TextRender|SetText (Variables|Default|GetText_TeleportMode) (Utilities|Text|ToText(String) (Utilities|String|EnumtoString _output_get)))
      (bind _asgame_instance (Utilities|Casting|CastToGameInstance (Game|GetGameInstance)))
      (Variables|/Game/VR_Player/Blueprints/GameInstance.GameInstance_C|SetTeleportMode _asgame_instance _output_get))
    (:ScaleMode
      (bind _asgame_state_2 (Utilities|Casting|CastToGameState (Game|GetGameState)))
      (bind _output_get_2 (Variables|/Game/VR_Player/Blueprints/VR_Character/GameState.GameState_C|SetScaleMode _asgame_state_2 (Utilities|Enum|ByteToEnumE_MoveMode (Math|Conversions|ToByte(Integer) (Math|Integer|%(Integer) (+ (Math|Conversions|ToInteger(Byte) (Variables|/Game/VR_Player/Blueprints/VR_Character/GameState.GameState_C|GetScaleMode _asgame_state_2)) 1) (|GetNumEnumEntries))))))
      (Rendering|Components|TextRender|SetText (Variables|Default|GetText_ScaleMode) (Utilities|Text|ToText(String) (Utilities|String|EnumtoString _output_get_2)))
      (bind _asgame_instance_2 (Utilities|Casting|CastToGameInstance (Game|GetGameInstance)))
      (Variables|/Game/VR_Player/Blueprints/GameInstance.GameInstance_C|SetScaleMode _asgame_instance_2 _output_get_2))
    (:ServerControlMode
      (bind _asgame_state_3 (Utilities|Casting|CastToGameState (Game|GetGameState)))
      (bind _output_get_3 (Variables|/Game/VR_Player/Blueprints/VR_Character/GameState.GameState_C|SetbServerControl _asgame_state_3 (not (Variables|/Game/VR_Player/Blueprints/VR_Character/GameState.GameState_C|GetbServerControl _asgame_state_3))))
      (Rendering|Components|TextRender|SetText (Variables|Default|GetText_ServerControl) (Utilities|Text|ToText(String) (Utilities|String|SelectString "On" "Off" _output_get_3)))
      (bind _asgame_instance_3 (Utilities|Casting|CastToGameInstance (Game|GetGameInstance)))
      (Variables|/Game/VR_Player/Blueprints/GameInstance.GameInstance_C|SetbServerControl _asgame_instance_3 _output_get_3))
    (:DragMode
      (bind _asgame_state_4 (Utilities|Casting|CastToGameState (Game|GetGameState)))
      (bind _output_get_4 (Variables|/Game/VR_Player/Blueprints/VR_Character/GameState.GameState_C|SetDragMode _asgame_state_4 (Utilities|Enum|ByteToEnumE_MoveMode (Math|Conversions|ToByte(Integer) (Math|Integer|%(Integer) (+ (Math|Conversions|ToInteger(Byte) (Variables|/Game/VR_Player/Blueprints/VR_Character/GameState.GameState_C|GetDragMode _asgame_state_4)) 1) (|GetNumEnumEntries))))))
      (Rendering|Components|TextRender|SetText (Variables|Default|GetText_DragMode) (Utilities|Text|ToText(String) (Utilities|String|EnumtoString _output_get_4)))
      (bind _asgame_instance_4 (Utilities|Casting|CastToGameInstance (Game|GetGameInstance)))
      (Variables|/Game/VR_Player/Blueprints/GameInstance.GameInstance_C|SetDragMode _asgame_instance_4 _output_get_4))))

(event EventBeginPlay
  (Utilities|FlowControl|Delay 1.0)
  (CallFunction|SetText))

(event EventTick
  (params (DeltaSeconds :type Float%20%28single-precision%29)))

(fn ConstructionScript)

(fn SetText
  (bind _asgame_state (Utilities|Casting|CastToGameState (Game|GetGameState)))
  (Utilities|FlowControl|Sequence
    (:then_0
      (Rendering|Components|TextRender|SetText (Variables|Default|GetText_TeleportMode) (Utilities|Text|ToText(String) (Utilities|String|EnumtoString (Variables|/Game/VR_Player/Blueprints/VR_Character/GameState.GameState_C|GetTeleportMode _asgame_state)))))
    (:then_1
      (Rendering|Components|TextRender|SetText (Variables|Default|GetText_ScaleMode) (Utilities|Text|ToText(String) (Utilities|String|EnumtoString (Variables|/Game/VR_Player/Blueprints/VR_Character/GameState.GameState_C|GetScaleMode _asgame_state)))))
    (:then_2
      (Rendering|Components|TextRender|SetText (Variables|Default|GetText_ServerControl) (Utilities|Text|ToText(String) (Utilities|String|SelectString "On" "Off" (Variables|/Game/VR_Player/Blueprints/VR_Character/GameState.GameState_C|GetbServerControl _asgame_state)))))
    (:then_3
      (Rendering|Components|TextRender|SetText (Variables|Default|GetText_DragMode) (Utilities|Text|ToText(String) (Utilities|String|EnumtoString (Variables|/Game/VR_Player/Blueprints/VR_Character/GameState.GameState_C|GetDragMode _asgame_state)))))))