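; VR GameState that drags, teleports and pivot-scales the world by transforming actors tagged "Move" or "Scalable", and rotates 4dObject actors.
; BeginPlay caches base transforms and copies mode settings from the GameInstance.
; Transforms apply relative to those baselines with per-actor tag speed multipliers (exponents when scaling), and ResetBaseTransform commits new baselines.
; Tick draws debug lines and fully connected network points, which follow these transforms.
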(event EventBeginPlay
  (Utilities|FlowControl|Delay 0.01)
  (Utilities|FlowControl|Sequence
    (:then_0
      (bind _outactors (Actor|GetAllActorswithTag "Scalable"))
      (bind _output_get (Variables|Default|SetWorldActorArray _outactors))
      (for (_array_element _array_index) _output_get
        (Utilities|Array|SetArrayElem (Variables|Default|GetBaseTransform) _array_index (Transformation|GetActorTransform _array_element) true)))
    (:then_1
      (bind _outactors_2 (Actor|GetAllActorswithTag "Move"))
      (bind _output_get_2 (Variables|Default|SetMoveableActors _outactors_2))
      (for (_array_element_2 _array_index_2) _output_get_2
        (Utilities|Array|SetArrayElem (Variables|Default|GetBaseMoveableTransform) _array_index_2 (Transformation|GetActorTransform _array_element_2) true)))
    (:then_2
      (bind _asgame_instance (Utilities|Casting|CastToGameInstance (Game|GetGameInstance)))
      (Variables|Default|SetTeleportMode (Variables|/Game/VR_Player/Blueprints/GameInstance.GameInstance_C|GetTeleportMode _asgame_instance))
      (Variables|Default|SetScaleMode (Variables|/Game/VR_Player/Blueprints/GameInstance.GameInstance_C|GetScaleMode _asgame_instance))
      (Variables|Default|SetDragMode (Variables|/Game/VR_Player/Blueprints/GameInstance.GameInstance_C|GetDragMode _asgame_instance))
      (Variables|Default|SetbServerControl (Variables|/Game/VR_Player/Blueprints/GameInstance.GameInstance_C|GetbServerControl _asgame_instance)))))

(event EventTick
  (params (DeltaSeconds :type Float%20%28single-precision%29))
  (bind _displaynetworkpoints (Variables|Default|GetDisplayNetworkPoints))
  (bind _displaynetworkpoints_2 (Variables|Default|GetDisplayNetworkPoints))
  (bind _returnvalue (Utilities|Array|Length _displaynetworkpoints))
  (if (Variables|Default|GetHasLines)
    (for (_array_element _array_index) (Variables|Default|GetDisplayDebugLineStart)
      (Rendering|Debug|DrawDebugLine _array_element (Utilities|Array|Get(acopy) (Variables|Default|GetDisplayDebugLineEnd) _array_index) (Variables|Default|GetLineColor) 0.0 (Utilities|Array|Get(acopy) (Variables|Default|GetDisplayLineWeights) _array_index)))
    (if (> _returnvalue 1)
      (for (_array_element_2 _array_index_2) (Variables|Default|GetDisplayNetworkPoints)
        (Rendering|Debug|DrawDebugPoint _array_element_2 15.0 "(R=0.000000,G=1.000000,B=1.000000,A=1.000000)" 0.0)
        (for _index (range _array_index_2 (- (Utilities|Array|Length _displaynetworkpoints_2) 1))
          (Rendering|Debug|DrawDebugLine :LineStart _array_element_2 :LineEnd (Utilities|Array|Get(acopy) _displaynetworkpoints_2 _index) :Thickness 0.0)))
      (elif (== _returnvalue 1)
        (Rendering|Debug|DrawDebugPoint (Utilities|Array|Get(acopy) (Variables|Default|GetDisplayNetworkPoints)) 15.0 "(R=0.000000,G=1.000000,B=1.000000,A=1.000000)" 0.0)))))

(fn ConstructionScript)

(fn MoveActors
  (params (T :type Vector))
  (bind _bdrag (Variables|Default|GetbDrag))
  (bind _returnvalue (Math|Vector|Equal(Vector) _bdrag "-1.000000,-1.000000,-1.000000" 0.0001))
  (LocalVariables|SetLocalTranslation (* T (Math|Vector|SelectVector "1.000000,1.000000,1.000000" _bdrag _returnvalue)))
  (Utilities|FlowControl|Sequence
    (:then_0
      (for (_array_element _array_index) (Variables|Default|GetMoveableActors)
        (if (or _returnvalue (== (Utilities|Array|FindItem (Variables|/Script/Engine.Actor|GetTags _array_element) "MoveSpeed") -1))
          (switch name (Utilities|Array|Get(acopy) (Variables|/Script/Engine.Actor|GetTags _array_element) 2)
            (:Default
              (LocalVariables|SetLocalSpeed 1.0))
            (:Fast
              (LocalVariables|SetLocalSpeed 2.0))
            (:Slow
              (LocalVariables|SetLocalSpeed 0.5)))
          (else
            (LocalVariables|SetLocalSpeed (Math|Conversions|ToFloat(Integer) (Utilities|String|ToString(Name) (Utilities|Array|Get(acopy) (Variables|/Script/Engine.Actor|GetTags _array_element) (+ (Utilities|Array|FindItem (Variables|/Script/Engine.Actor|GetTags _array_element) "MoveSpeed") 1)))))))
        (Transformation|SetActorLocation _array_element (+ (.Location (Math|Transform|BreakTransform (Utilities|Array|Get(acopy) (Variables|Default|GetBaseMoveableTransform) _array_index))) (* (LocalVariables|GetLocalTranslation) (LocalVariables|GetLocalSpeed))) false false)))
    (:then_1
      (if (Variables|Default|GetMoveLines)
        (for (_array_element_2 _array_index_2) (Variables|Default|GetBaseDebugLineStart)
          (Utilities|Array|SetArrayElem (Variables|Default|GetDisplayDebugLineStart) _array_index_2 (+ _array_element_2 (LocalVariables|GetLocalTranslation)))
          (Utilities|Array|SetArrayElem (Variables|Default|GetDisplayDebugLineEnd) _array_index_2 (+ (Utilities|Array|Get(acopy) (Variables|Default|GetBaseDebugLineEnd) _array_index_2) (LocalVariables|GetLocalTranslation))))))
    (:then_2
      ;[1 1 1] Network Points
      (for (_array_element_3 _array_index_3) (Variables|Default|GetBasetNetworkPoints)
        (Utilities|Array|SetArrayElem (Variables|Default|GetDisplayNetworkPoints) _array_index_3 (+ _array_element_3 (LocalVariables|GetLocalTranslation)))))))

(fn ScaleActors
  (params (Pivot :type Vector) (Scale :type Float%20%28single-precision%29))
  (LocalVariables|SetLocalPivot Pivot)
  (LocalVariables|SetLocalScale (Math|Float|Power Scale (Variables|Default|GetScaleSpeed)))
  (Variables|Default|SetDisplayScale (* (LocalVariables|GetLocalScale) (Variables|Default|GetBaseScale)))
  (Variables|Default|SetDisplayPivot Pivot)
  (Utilities|FlowControl|Sequence
    (:then_0
      (for (_array_element _array_index) (Variables|Default|GetWorldActorArray)
        (if (!= (Utilities|Array|FindItem (Variables|/Script/Engine.Actor|GetTags _array_element) "ScaleSpeed") -1)
          (LocalVariables|SetLocalExp (Math|Conversions|ToFloat(Integer) (Utilities|String|ToString(Name) (Utilities|Array|Get(acopy) (Variables|/Script/Engine.Actor|GetTags _array_element) (+ (Utilities|Array|FindItem (Variables|/Script/Engine.Actor|GetTags _array_element) "ScaleSpeed") 1)))))
          (else
            (switch name (Utilities|Array|Get(acopy) (Variables|/Script/Engine.Actor|GetTags _array_element) 2)
              (:Default
                (LocalVariables|SetLocalExp 1.0))
              (:Fast
                (LocalVariables|SetLocalExp 2.0))
              (:Slow
                (LocalVariables|SetLocalExp 0.5)))))
        (Transformation|SetActorTransform _array_element (Math|Transform|MakeTransform (Utilities|Scale (.Location (Math|Transform|BreakTransform (Utilities|Array|Get(acopy) (Variables|Default|GetBaseTransform) _array_index))) (LocalVariables|GetLocalPivot) (Math|Float|Power (LocalVariables|GetLocalScale) (LocalVariables|GetLocalExp))) (.Rotation (Math|Transform|BreakTransform (Utilities|Array|Get(acopy) (Variables|Default|GetBaseTransform) _array_index))) (* (.Scale (Math|Transform|BreakTransform (Utilities|Array|Get(acopy) (Variables|Default|GetBaseTransform) _array_index))) (Math|Float|Power (LocalVariables|GetLocalScale) (LocalVariables|GetLocalExp)))) false true)))
    (:then_1
      (if (Variables|Default|GetScaleLines)
        (for (_array_element_2 _array_index_2) (Variables|Default|GetBaseDebugLineStart)
          (Utilities|Array|SetArrayElem (Variables|Default|GetDisplayDebugLineStart) _array_index_2 (Utilities|Scale _array_element_2 (LocalVariables|GetLocalPivot) (LocalVariables|GetLocalScale)))
          (Utilities|Array|SetArrayElem (Variables|Default|GetDisplayDebugLineEnd) _array_index_2 (Utilities|Scale (Utilities|Array|Get(acopy) (Variables|Default|GetBaseDebugLineEnd) _array_index_2) (LocalVariables|GetLocalPivot) (LocalVariables|GetLocalScale)))
          (Utilities|Array|SetArrayElem (Variables|Default|GetDisplayLineWeights) _array_index_2 (Math|Float|SelectFloat (* (Utilities|Array|Get(acopy) (Variables|Default|GetBaseLineWeights) _array_index_2) (LocalVariables|GetLocalScale)) (Utilities|Array|Get(acopy) (Variables|Default|GetBaseLineWeights) _array_index_2) (Variables|Default|GetScaleLineWeights))))))
    (:then_2
      (for (_array_element_3 _array_index_3) (Variables|Default|GetBasetNetworkPoints)
        (Utilities|Array|SetArrayElem (Variables|Default|GetDisplayNetworkPoints) _array_index_3 (Utilities|Scale _array_element_3 (LocalVariables|GetLocalPivot) (LocalVariables|GetLocalScale)))))))

(fn ResetBaseTransform
  (Utilities|FlowControl|Sequence
    (:then_0
      (for (_array_element _array_index) (Variables|Default|GetWorldActorArray)
        (Utilities|Array|SetArrayElem (Variables|Default|GetBaseTransform) _array_index (Transformation|GetActorTransform _array_element))))
    (:then_1
      (bind _outactors (Actor|GetAllActorswithTag "Move"))
      (bind _output_get (Variables|Default|SetMoveableActors _outactors))
      (for (_array_element_2 _array_index_2) _output_get
        (Utilities|Array|SetArrayElem (Variables|Default|GetBaseMoveableTransform) _array_index_2 (Transformation|GetActorTransform _array_element_2) true)))
    (:then_2
      (Variables|Default|SetBaseDebugLineStart (Variables|Default|GetDisplayDebugLineStart))
      (Variables|Default|SetBaseDebugLineEnd (Variables|Default|GetDisplayDebugLineEnd))
      (Variables|Default|SetBaseLineWeights (Variables|Default|GetDisplayLineWeights))
      (Variables|Default|SetBaseScale (Variables|Default|GetDisplayScale))
      (Variables|Default|SetBasePivot (Variables|Default|GetDisplayPivot))
      (Variables|Default|SetBasetNetworkPoints (Variables|Default|GetDisplayNetworkPoints)))
    (:then_3
      (if (Variables|Default|GetScaleDragSpeed)
        (Variables|Default|SetDragSpeed (Variables|Default|GetDisplayScale))))))

(fn SetDebugLineTransform
  (params (LineStart :type Array%20of%20Vectors) (LineEnd :type Array%20of%20Vectors) (LineWeight :type Array%20of%20Floats%20%28single-precision%29))
  (Variables|Default|SetDisplayDebugLineStart LineStart)
  (Variables|Default|SetDisplayDebugLineEnd LineEnd)
  (Variables|Default|SetDisplayLineWeights LineWeight)
  (Variables|Default|SetBaseLineWeights LineWeight)
  (Variables|Default|SetBaseDebugLineStart LineStart)
  (Variables|Default|SetBaseDebugLineEnd LineEnd))

(fn TeleportActors
  (params (T :type Vector))
  (LocalVariables|SetLocalTranslation (* T (Variables|Default|GetbTeleport)))
  (Utilities|FlowControl|Sequence
    (:then_0
      (for (_array_element _array_index) (Variables|Default|GetMoveableActors)
        (switch name (Utilities|Array|Get(acopy) (Variables|/Script/Engine.Actor|GetTags _array_element) 2)
          (:Default
            (LocalVariables|SetLocalSpeed 1.0))
          (:Fast
            (LocalVariables|SetLocalSpeed 2.0))
          (:Slow
            (LocalVariables|SetLocalSpeed 0.5)))
        (Transformation|SetActorLocation _array_element (+ (.Location (Math|Transform|BreakTransform (Utilities|Array|Get(acopy) (Variables|Default|GetBaseMoveableTransform) _array_index))) (* (LocalVariables|GetLocalTranslation) (LocalVariables|GetLocalSpeed))) false false)))
    (:then_1
      (if (Variables|Default|GetMoveLines)
        (for (_array_element_2 _array_index_2) (Variables|Default|GetBaseDebugLineStart)
          (Utilities|Array|SetArrayElem (Variables|Default|GetDisplayDebugLineStart) _array_index_2 (+ _array_element_2 (LocalVariables|GetLocalTranslation)))
          (Utilities|Array|SetArrayElem (Variables|Default|GetDisplayDebugLineEnd) _array_index_2 (+ (Utilities|Array|Get(acopy) (Variables|Default|GetBaseDebugLineEnd) _array_index_2) (LocalVariables|GetLocalTranslation))))))
    (:then_2
      ;[1 1 1] Network Points
      (for (_array_element_3 _array_index_3) (Variables|Default|GetBasetNetworkPoints)
        (Utilities|Array|SetArrayElem (Variables|Default|GetDisplayNetworkPoints) _array_index_3 (+ _array_element_3 (LocalVariables|GetLocalTranslation)))))))

(fn SetActorLocation
  (params (ActorRef :type Actor%20Object%20Reference) (NewLocation :type Vector))
  (bind _moveableactors (Variables|Default|GetMoveableActors))
  (bind _basemoveabletransform (Variables|Default|GetBaseMoveableTransform))
  (bind _returnvalue (Utilities|Array|FindItem _moveableactors ActorRef))
  (bind _item (Utilities|Array|Get(acopy) _basemoveabletransform _returnvalue))
  (bind (_location _rotation _scale) (Math|Transform|BreakTransform _item))
  (Utilities|Array|SetArrayElem _basemoveabletransform _returnvalue (Math|Transform|MakeTransform (- NewLocation (- (.Location (Math|Transform|BreakTransform (Transformation|GetActorTransform ActorRef))) _location)) _rotation _scale)))

(fn SetActorBaseTransform
  (params (Actor :type 4d%20Point%20Actor%20Object%20Reference))
  (Utilities|Array|SetArrayElem (Variables|Default|GetBaseMoveableTransform) (Utilities|Array|FindItem (Variables|Default|GetMoveableActors) Actor) (Transformation|GetActorTransform Actor)))

(fn Rotate4DActors
  (params (R :type Rotator) (L :type Rotator))
  (bind (_roll _pitch) (Math|Rotator|BreakRotator R))
  (bind (_roll_2 _pitch_2) (Math|Rotator|BreakRotator L))
  (bind _outactors (Actor|GetAllActorsOfClass "/Game/BluePrints/4d/4dObject.4dObject_C"))
  (Default|Rotate _outactors "NewEnumerator0" (Utilities|RotationTransform _roll))
  (Default|Rotate _outactors "NewEnumerator1" (Utilities|RotationTransform _pitch))
  (Default|Rotate _outactors "NewEnumerator5" (Utilities|RotationTransform _roll_2))
  (Default|Rotate _outactors "NewEnumerator3" (Utilities|RotationTransform _pitch_2)))

(fn SpawnLine
  (params (Location1 :type Vector) (Location2 :type Vector)))