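; CameraRecorder is an actor that saves what its SceneCaptureComponent2D sees as a numbered sequence of image files.
; While Record is true, Tick accumulates delta time and exports a shot whenever the 1/FPS interval is exceeded, then resets the timer to zero.
; TakeSingleShot triggers the same export on demand, incrementing FrameCount and writing the render target to FilePath with a prefix, counter and extension.
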(event Custom|TakeSingleShot
  (Math|Integer|IncrementInt (Variables|Default|GetFrameCount)
    (:%20%20
      (Rendering|ExportRenderTarget (Variables|/Script/Engine.SceneCaptureComponent2D|GetTextureTarget (Variables|Default|GetSceneCaptureComponent2D)) (Variables|Default|GetFilePath) (Utilities|String|Append (Variables|Default|GetFilePrefix) (Utilities|String|ToString(Integer) (Variables|Default|GetFrameCount)) (Variables|Default|GetFileExtension))))))

(event EventBeginPlay)

(event Collision|EventActorBeginOverlap
  (params (OtherActor :type Actor%20Object%20Reference)))

(event EventTick
  (params (DeltaSeconds :type Float%20%28single-precision%29))
  (if (Variables|Default|GetbRecord)
    (bind _output_get (Variables|Default|SetTimer (+ DeltaSeconds (Variables|Default|GetTimer))))
    (if (> _output_get (/ 1.0 (Variables|Default|GetFPS)))
      (Variables|Default|SetTimer 0.0)
      (Math|Integer|IncrementInt (Variables|Default|GetFrameCount)
        (:%20%20
          (Rendering|ExportRenderTarget (Variables|/Script/Engine.SceneCaptureComponent2D|GetTextureTarget (Variables|Default|GetSceneCaptureComponent2D)) (Variables|Default|GetFilePath) (Utilities|String|Append (Variables|Default|GetFilePrefix) (Utilities|String|ToString(Integer) (Variables|Default|GetFrameCount)) (Variables|Default|GetFileExtension))))))))

(fn ConstructionScript)