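; VR game instance with logic to export head and hand position logs to text files, currently disconnected from any event.
; The unwired chain flattens the HMD, left-hand and right-hand string arrays through ArrayToString, which concatenates without a separator.
; FileSaveString would write each result under Saved\PositionTracking with a date-time filename and device suffix.
; The Shutdown event is empty, and nothing here fills the arrays.
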(event EventShutdown)

(fn ArraytoString
  (params (Array :type Array%20of%20Strings))
  (for _array_element Array
    (LocalVariables|SetLocalString (Utilities|String|Append (LocalVariables|GetLocalString) _array_element " 
")))
  (return (LocalVariables|GetLocalString)))